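; Base RTS unit Blueprint that handles team setup, stance orders and attack commands.
; BeginPlay polls until owner and team are valid, then copies the team index; team 1 gets red material and an in-game UI widget.
; SiebarthOrder's OnRep applies stances: aggro sphere on/off, movement toggle for Hold Position, or stop.
; Sphere overlaps and AttackTarget issue AI attack orders; health changes with a valid damage causer reset the stance to None.
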(event OnComponentBeginOverlap(Sphere)
  (params (OverlappedComponent :type Primitive%20Component%20Object%20Reference) (OtherActor :type Actor%20Object%20Reference) (OtherComp :type Primitive%20Component%20Object%20Reference) (OtherBodyIndex :type Integer) (bFromSweep :type Boolean) (SweepResult :type Hit%20Result%20Structure%20%28by%20ref%29))
  (if (Variables|Default|GetIsAggressiv)
    (if (not (Class|RTSOwnerComponent|IsSameTeamasActor (Variables|Default|GetRTSOwner) OtherActor))
      (bind _output_get (Variables|Default|SetOther%20Actor OtherActor))
      (Utilities|IsValid (Actor|GetComponentbyClass _output_get "/Script/RealTimeStrategy.RTSHealthComponent")
        (:Is%20Valid
          (bind _asrtspawn_aicontroller (Utilities|Casting|CastToRTSPawnAIController (Pawn|GetController)))
          (Class|RTSPawnAIController|IssueStopOrder _asrtspawn_aicontroller)
          (Class|RTSPawnAIController|IssueAttackOrder _asrtspawn_aicontroller (Variables|Default|GetOther%20Actor)))))))

(event OnHealthChanged(RTSHealth)
  (params (Actor :type Actor%20Object%20Reference) (OldHealth :type Float%20%28single-precision%29) (NewHealth :type Float%20%28single-precision%29) (DamageCauser :type Actor%20Object%20Reference))
  (Utilities|IsValid DamageCauser
    (:Is%20Valid
      (Variables|Default|SetSiebarthOrder_ "NewEnumerator0"))))

(event EventAttackTarget
  (params (Hit :type Hit%20Result%20Structure))
  (bind _asrtspawn_aicontroller (Utilities|Casting|CastToRTSPawnAIController (Pawn|GetController)))
  (Class|RTSPawnAIController|IssueStopOrder _asrtspawn_aicontroller)
  (Class|RTSPawnAIController|IssueAttackOrder _asrtspawn_aicontroller (.HitActor (Collision|BreakHitResult Hit))))

(event EventBeginPlay
  (bind _rtsowner (Variables|Default|GetRTSOwner))
  (bind _returnvalue (Class|RTSOwnerComponent|GetPlayerOwner _rtsowner))
  (bind _returnvalue_2 (Class|RTSPlayerState|GetTeam _returnvalue))
  (bind _returnvalue_3 (Class|RTSTeamInfo|GetTeamIndex _returnvalue_2))
  (Utilities|FlowControl|Sequence
    (:then_0
      (Utilities|IsValid _returnvalue :!label _label
        (:Is%20Valid
          (Utilities|IsValid _returnvalue_2 :!label _label_2
            (:Is%20Valid
              (Variables|/Script/RealTimeStrategy.RTSSelectableComponent|SetTEAMINDEX (Variables|Default|GetRTSSelectable) _returnvalue_3)
              (switch string (Utilities|String|ToString(Byte) _returnvalue_3)
                (:1
                  (Rendering|Material|SetMaterial (Variables|Character|GetMesh) 0 "/Game/Toony_Tiny_RTS_Set_UE5/Materials/Units/MI_Units_Red.MI_Units_Red")
                  (bind _returnvalue_4 (UserInterface|CreateWidget "/Game/UI/Widgets/WBP_IngameUI.WBP_IngameUI_C" (Game|GetPlayerController 0)))
                  (Variables|Default|SetIngameUI _returnvalue_4))))
            (:Is%20Not%20Valid
              (Utilities|FlowControl|Delay 0.5)
              (goto _label_2))))
        (:Is%20Not%20Valid
          (Utilities|FlowControl|Delay 0.5)
          (goto _label))))))

(event EventSiebarthOrder
  (params (SiebarthOrder :type SiebarthOrders%20Enum :default "NewEnumerator0"))
  (Variables|Default|SetSiebarthOrder_ SiebarthOrder))

(fn ConstructionScript)

(fn OnRepSiebarthOrder
  (bind _charactermovement (Variables|Character|GetCharacterMovement))
  (bind _sphere (Variables|Default|GetSphere))
  (switch Utilities|FlowControl|Switch|SwitchonSiebarthOrders (Variables|Default|GetSiebarthOrder_)
    (:NewEnumerator0
      (Variables|Default|SetIsAggressiv false)
      (Collision|SetCollisionEnabled _sphere "NoCollision"))
    (:NewEnumerator1
      (Variables|Default|SetIsAggressiv true)
      (Collision|SetCollisionEnabled _sphere "QueryOnly"))
    (:NewEnumerator4
      (if (Variables|Default|GetCanMove)
        (Variables|Default|SetCanMove false)
        (Components|Activation|Deactivate _charactermovement)
        (else
          (Variables|Default|SetCanMove true)
          (Components|Activation|Activate _charactermovement false))))
    (:NewEnumerator5
      (bind _asrtspawn_aicontroller (Utilities|Casting|CastToRTSPawnAIController (Pawn|GetController)))
      (Class|RTSPawnAIController|IssueStopOrder _asrtspawn_aicontroller))))