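; Infantry building Blueprint for an RTS that tints its mesh to match the owning player's team.
; On BeginPlay it polls the RTSOwner component every half second until the player owner, then its team, is valid.
; It then switches on the team index as a string, with only team 1 handled, which gets the red building material on the static mesh.
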(event EventBeginPlay
  (bind _rtsowner (Variables|Default|GetRTSOwner))
  (bind _returnvalue (Class|RTSOwnerComponent|GetPlayerOwner _rtsowner))
  (bind _returnvalue_2 (Class|RTSPlayerState|GetTeam _returnvalue))
  (Utilities|IsValid _returnvalue :!label _label
    (:Is%20Valid
      (Utilities|IsValid _returnvalue_2 :!label _label_2
        (:Is%20Valid
          (switch string (Utilities|String|ToString(Byte) (Class|RTSTeamInfo|GetTeamIndex _returnvalue_2))
            (:1
              (Rendering|Material|SetMaterial (Variables|Default|GetStaticMesh) 0 "/Game/Toony_Tiny_RTS_Set_UE5/Materials/Buildings/MI_Buildings_Red.MI_Buildings_Red"))))
        (:Is%20Not%20Valid
          (Utilities|FlowControl|Delay 0.5)
          (goto _label_2))))
    (:Is%20Not%20Valid
      (Utilities|FlowControl|Delay 0.5)
      (goto _label))))

(fn ConstructionScript)