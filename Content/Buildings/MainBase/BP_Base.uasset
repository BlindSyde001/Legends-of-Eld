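; Main base building for an RTS that applies its team identity, positions builder units and displays a production rally point.
; On BeginPlay it polls until owner and team are valid, then sets the selectable's team index and swaps to red material for team 1.
; Same-team builders move to five StartSpawn points, chosen by their index among all builders.
; The rally marker shows while selected, following RTSProduction's rally point on selection or after SendRightClick.
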(event OnSelected(RTSSelectable)
  (params (Actor :type Actor%20Object%20Reference))
  (bind _rtsproduction (Variables|Default|GetRTSProduction))
  (bind _rallypoint (Variables|Default|GetRallyPoint))
  (bind _returnvalue (Class|RTSProductionComponent|GetRallyPoint _rtsproduction))
  (bind _targetlocation (Utilities|Struct|BreakRTSProductionRallyPoint _returnvalue))
  (Rendering|SetVisibility _rallypoint true false)
  (Transformation|SetWorldLocation _rallypoint (Math|Vector|MakeVector (.x _targetlocation) (.y _targetlocation) (.z (Transformation|GetWorldLocation _rallypoint))) false false))

(event OnDeselected(RTSSelectable)
  (params (Actor :type Actor%20Object%20Reference))
  (Rendering|SetVisibility (Variables|Default|GetRallyPoint) false false))

(event EventBeginPlay
  (bind _rtsowner (Variables|Default|GetRTSOwner))
  (bind _returnvalue (Class|RTSOwnerComponent|GetPlayerOwner _rtsowner))
  (bind _returnvalue_2 (Class|RTSPlayerState|GetTeam _returnvalue))
  (bind _returnvalue_3 (Class|RTSTeamInfo|GetTeamIndex _returnvalue_2))
  (Utilities|IsValid _returnvalue :!label _label
    (:Is%20Valid
      (Utilities|IsValid _returnvalue_2 :!label _label_2
        (:Is%20Valid
          (Utilities|FlowControl|Sequence
            (:then_0
              (Variables|/Script/RealTimeStrategy.RTSSelectableComponent|SetTEAMINDEX (Variables|Default|GetRTSSelectable) _returnvalue_3)
              (switch string (Utilities|String|ToString(Byte) _returnvalue_3)
                (:1
                  (Rendering|Material|SetMaterial (Variables|Default|GetStaticMesh) 0 "/Game/Toony_Tiny_RTS_Set_UE5/Materials/Buildings/MI_Buildings_Red.MI_Buildings_Red"))))
            (:then_1
              (bind _outactors (Actor|GetAllActorsOfClass "/Game/Units/CMV/BP_Unit_Builder.BP_Unit_Builder_C"))
              (for (_array_element _array_index) _outactors
                (if (Class|RTSOwnerComponent|IsSameTeamasActor (Variables|Default|GetRTSOwner) _array_element)
                  (switch int _array_index
                    (:0
                      (Utilities|NewMacro _array_element (Variables|Default|GetStartSpawn)))
                    (:1
                      (Utilities|NewMacro _array_element (Variables|Default|GetStartSpawn1)))
                    (:2
                      (Utilities|NewMacro _array_element (Variables|Default|GetStartSpawn2)))
                    (:3
                      (Utilities|NewMacro _array_element (Variables|Default|GetStartSpawn3)))
                    (:4
                      (Utilities|NewMacro _array_element (Variables|Default|GetStartSpawn4)))))))))
        (:Is%20Not%20Valid
          (Utilities|FlowControl|Delay 0.5)
          (goto _label_2))))
    (:Is%20Not%20Valid
      (Utilities|FlowControl|Delay 0.5)
      (goto _label))))

(event EventSendRightClick
  (bind _rtsproduction (Variables|Default|GetRTSProduction))
  (bind _rallypoint (Variables|Default|GetRallyPoint))
  (bind _returnvalue (Class|RTSProductionComponent|GetRallyPoint _rtsproduction))
  (bind _targetlocation (Utilities|Struct|BreakRTSProductionRallyPoint _returnvalue))
  (Utilities|FlowControl|Delay 0.2)
  (Transformation|SetWorldLocation _rallypoint (Math|Vector|MakeVector (.x _targetlocation) (.y _targetlocation) (.z (Transformation|GetWorldLocation _rallypoint))) false false))

(fn ConstructionScript)